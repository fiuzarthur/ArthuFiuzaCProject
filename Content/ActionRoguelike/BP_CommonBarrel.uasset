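; BP_CommonBarrel is a short-lived barrel actor that awards score when the player destroys it.
; It destroys itself four seconds after BeginPlay.
; On Destroyed, if the DestroyByPlayer flag is set, it increments Score on the player character and spawns an explosion emitter slightly above its location.
; The flag is only read here, so timed removal gives no score or effect unless it has been set.
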(event EventBeginPlay
  (Utilities|FlowControl|Delay 4.0)
  (Actor|DestroyActor))

(event EventDestroyed
  (bind _returnvalue (Transformation|GetActorLocation))
  (bind (_x _y _z) (Math|Vector|BreakVector _returnvalue))
  (if (Variables|Default|GetdestroyByPlayer)
    (bind _asbp_player_character (Utilities|Casting|CastToBP_Player_Character (Game|GetPlayerCharacter 0)))
    (Math|Integer|IncrementInt (Variables|/Game/ActionRoguelike/BP_Player_Character.BP_Player_Character_C|GetScore _asbp_player_character)
      (:%20%20
        (Effects|SpawnEmitteratLocation "/Game/ExampleContent/Effects/P_Explosion.P_Explosion" (Math|Vector|MakeVector _x _y (+ _z 1e+02)) (Transformation|GetActorRotation))))))

(fn ConstructionScript)